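; GlobalInstance holds game-wide progression for what appears to be a Christmas-themed game: chimney, visual and present unlocks, score, maps and completed days.
; LoadStats copies supplied save values into these variables, except in November, when it zeroes all progress and the current map, then saves through BP_SaveDataActor.
; Main menu open and close events set the menu flag and block or allow spawning on the Spawner.
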(event Custom|OpenMainMenu
  (Variables|Default|SetShowMainMenu true)
  (Default|Don'tAllowSpawning (Variables|Default|GetSpawner)))

(event Custom|CloseMainMenu
  (Variables|Default|SetShowMainMenu false)
  (Default|AllowSpawning (Variables|Default|GetSpawner)))

(event Custom|LoadStats
  (params (Chimney :type Integer) (Visuals :type Integer) (Score :type Integer) (Maps :type Integer) (Completed :type Integer) (PresentUnlocks :type Integer))
  (if (== (Class|KismetMathLibrary|GetMonth (Class|KismetMathLibrary|Today)) 11)
    (Variables|Default|SetChimneyUnlocks 0)
    (Variables|Default|SetVisualUpgrades 0)
    (Variables|Default|SetSavedScore 0)
    (Variables|Default|SetMapsUnlocked 0)
    (Variables|Default|SetCompletedDays 0)
    (Variables|Default|SetPresentUnlocks 0)
    (Variables|Default|SetCurrentMap 0)
    (bind _outactors (Actor|GetAllActorsOfClass "/Game/Blueprints/Calendar/SavingAndWidgets/BP_SaveDataActor.BP_SaveDataActor_C"))
    (Default|SaveGame _outactors)
    (else
      (Variables|Default|SetChimneyUnlocks Chimney)
      (Variables|Default|SetVisualUpgrades Visuals)
      (Variables|Default|SetSavedScore Score)
      (Variables|Default|SetMapsUnlocked Maps)
      (Variables|Default|SetCompletedDays Completed)
      (Variables|Default|SetPresentUnlocks PresentUnlocks))))
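; Blueprint that pushes gift objects sideways with a randomly varying wind.
; While the Wind flag is on, Tick calls ApplyWind, which adds WindForce to the Paper Sprite component of every actor tagged "Gift", searching for them each frame.
; SetWind picks a random force along X and re-arms itself on a random timer; nothing in this file makes the first SetWind call.
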(event Custom|Apply%20Wind
  ;[1 1 1] Apply Wind
  (bind _outactors (Actor|GetAllActorswithTag "Gift"))
  (for _array_element _outactors
    (Physics|AddForce (Actor|GetComponentbyClass _array_element "/Script/Paper2D.PaperSpriteComponent") (Variables|Default|GetWindForce) "None" false)))

(event Custom|Set%20Wind
  ;[1 1 1] Set Wind
  (Variables|Default|SetWindForce (Math|Vector|MakeVector (Math|Random|RandomFloatinRange (Variables|Default|GetMinWind) (Variables|Default|GetMaxWind)) 0.0 0.0))
  (Utilities|Time|SetTimerbyEvent (delegate Custom|Set%20Wind) (Math|Random|RandomFloatinRange 1.0 5.0)))

(event EventTick
  (params (DeltaSeconds :type Float%20%28single-precision%29))
  (if (Variables|Default|GetWind)
    (CallFunction|ApplyWind)))

(fn ConstructionScript)
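; Gift actor that can be redirected by a touch swipe once Enable turns its input on.
; Swiping past a threshold slows global time and draws a predicted ballistic arc with particle emitters each tick.
; Release replaces the gift's velocity with a clamped swipe impulse, restores time and disables input.
; The first hit also disables input, notifying AudioManager for surfaces tagged Sides, and destruction restores normal time.
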(event Custom|DrawAim
  (bind _returnvalue (Game|GetPlayerController 0))
  (bind _beginloc (Variables|Default|GetBeginLoc))
  (bind (_locationx _locationy _biscurrentlypressed) (Class|PlayerController|GetInputTouchState _returnvalue "Touch1"))
  (bind _returnvalue_2 (Math|Conversions|ToVector(Vector2D) _beginloc))
  (bind _returnvalue_3 (Math|Vector2D|MakeVector2D _locationx _locationy))
  (bind _returnvalue_4 (Math|Conversions|ToVector(Vector2D) _returnvalue_3))
  (bind _returnvalue_5 (- _returnvalue_2 _returnvalue_4))
  (bind _returnvalue_6 (* _returnvalue_5 -1.0))
  (bind _returnvalue_7 (Math|Vector|ClampVectorSize _returnvalue_6 0.0 1.7e+02))
  (bind (_x _y _z) (Math|Vector|BreakVector _returnvalue_7))
  ;[1 1 1] Draw Aim
  (bind _index (Utilities|FlowControl|ForLoopwithBreak 0 (Math|Float|Floor (/ (Variables|Default|GetPathLifeTime) (Variables|Default|GetTimeInterval))))
    (:LoopBody
      (bind (_point1 _point2) (CallFunction|GetSegmentatTime (Transformation|GetActorLocation) (Math|Vector|MakeVector _x _z (* _y -1.0)) "0, 0,-350.000000" (* _index (Variables|Default|GetTimeInterval)) (* (+ _index 1) (Variables|Default|GetTimeInterval))))
      (Collision|LineTraceByChannel _point1 _point2 "TraceTypeQuery1" true 0 "None" true "(R=0.000000,G=0.000000,B=0.000000,A=0.000000)" "(R=0.000000,G=1.000000,B=0.000000,A=0.000000)")
      (bind _returnvalue_8 (Effects|SpawnEmitteratLocation "/Game/Particles/P_Aiming_02.P_Aiming_02" _point1 "0, 0, 0" "0.300000,0.300000,0.300000"))
      (Rendering|SetTranslucentSortPriority _returnvalue_8 50))))

(event Custom|Enable
  ;[1 1 1] Event BeginPlay and EventTick
  (Input|EnableInput (Game|GetPlayerController 0)))

(event EventBeginPlay
  ;[1 1 1] Event BeginPlay and EventTick
)

(event EventTick
  (params (DeltaSeconds :type Float%20%28single-precision%29))
  (bind _returnvalue (Game|GetPlayerController 0))
  (bind (_locationx _locationy _biscurrentlypressed) (Class|PlayerController|GetInputTouchState _returnvalue "Touch1"))
  (bind _returnvalue_2 (Math|Vector2D|MakeVector2D _locationx _locationy))
  ;[1 1 1] Event BeginPlay and EventTick
  ;[1 1 1] Swipe
  (Utilities|FlowControl|Gate true
    (:Exit
      (if (>= (Math|Vector2D|Vector2DLength (- _returnvalue_2 (stale Input|ActionEvents|InputActionFinger1 _output_get))) (Variables|Default|GetSwipeThresh))
        (CallFunction|DrawAim)
        (Utilities|Time|SetGlobalTimeDilation 0.05)
        (Variables|Default|SetStartLoc "(X=100000.000000,Y=100000.000000)")
        (Variables|Default|SetPriorLoc _returnvalue_2)))))

(event Collision|EventHit
  (params (MyComp :type Primitive%20Component%20Object%20Reference) (Other :type Actor%20Object%20Reference) (OtherComp :type Primitive%20Component%20Object%20Reference) (bSelfMoved :type Boolean) (HitLocation :type Vector :default "0, 0, 0") (HitNormal :type Vector :default "0, 0, 0") (NormalImpulse :type Vector :default "0, 0, 0") (Hit :type Hit%20Result%20Structure%20%28by%20ref%29))
  (Utilities|FlowControl|DoOnce false
    (:Completed
      (Input|DisableInput 0)
      (if (Components|ComponentHasTag (.HitComponent (Collision|BreakHitResult Hit)) "Sides")
        (bind _outactors (Actor|GetAllActorsOfClass "/Game/Blueprints/Main/AudioManager.AudioManager_C"))
        (Default|SideHit _outactors)))))

(event EventDestroyed
  (Input|DisableInput 0)
  (Utilities|Time|SetGlobalTimeDilation 1.0))

(event Input|ActionEvents|InputActionFinger1
  (params (Key :type Key%20Structure))
  (bind _returnvalue (Game|GetPlayerController 0))
  (bind (_locationx _locationy _biscurrentlypressed) (Class|PlayerController|GetInputTouchState _returnvalue "Touch1"))
  (bind _returnvalue_2 (Math|Vector2D|MakeVector2D _locationx _locationy))
  ;[1 1 1] Swipe
  (:Pressed
    (bind _output_get (Variables|Default|SetStartLoc _returnvalue_2))
    (bind _output_get_2 (Variables|Default|SetBeginLoc _returnvalue_2))
    (Variables|Default|SetPriorLoc _output_get)
    (Utilities|FlowControl|Gate true) ; enters at Open
  )
  (:Released
    (Utilities|FlowControl|Sequence
      (:then_0
        (Utilities|FlowControl|Gate true) ; enters at Close
      )
      (:then_1
        (if (not _biscurrentlypressed)
          (if (not (Math|Vector|Equal(Vector) (Variables|Default|GetStartLoc) (Variables|Default|GetPriorLoc) 0.0001))
            (Variables|Default|SetReleaseLoc _returnvalue_2)
            (Variables|Default|SetLatestImpulse (Math|Vector|MakeVector (.X (Math|Vector|BreakVector (Math|Vector|ClampVectorSize (* (- (Math|Conversions|ToVector(Vector2D) _output_get_2) (Math|Conversions|ToVector(Vector2D) (Variables|Default|GetReleaseLoc))) -1.0) 0.0 1.7e+02))) (.Z (Math|Vector|BreakVector (Math|Vector|ClampVectorSize (* (- (Math|Conversions|ToVector(Vector2D) _output_get_2) (Math|Conversions|ToVector(Vector2D) (Variables|Default|GetReleaseLoc))) -1.0) 0.0 1.7e+02))) (* (.Y (Math|Vector|BreakVector (Math|Vector|ClampVectorSize (* (- (Math|Conversions|ToVector(Vector2D) _output_get_2) (Math|Conversions|ToVector(Vector2D) (Variables|Default|GetReleaseLoc))) -1.0) 0.0 1.7e+02))) -1.0)))
            ;[1 1 1] Create gift and add force to it depending on the swipe length
            (Physics|SetPhysicsLinearVelocity (Variables|Default|GetRenderComponent) "0, 0, 0" false "None")
            (Physics|AddImpulse (Actor|GetComponentbyClass "/Script/Paper2D.PaperSpriteComponent") (Variables|Default|GetLatestImpulse) "None" true)
            (Input|DisableInput 0)
            (Utilities|Time|SetGlobalTimeDilation 1.0)
            (Variables|Default|SetPriorLoc _returnvalue_2)))))))

(fn ConstructionScript)

(fn GetSegmentatTime
  (params (StartLoc :type Vector) (Impulse :type Vector) (Gravity :type Vector) (Time1 :type Float%20%28single-precision%29) (Time2 :type Float%20%28single-precision%29))
  (return (+ StartLoc (* Impulse Time1) (* Gravity (* Time1 Time1 0.5))) (+ StartLoc (* Impulse Time2) (* Gravity (* Time2 Time2 0.5)))))
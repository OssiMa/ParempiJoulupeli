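; Present gift actor that shows a randomly chosen Paper2D sprite and reports its first impact for audio feedback.
; On BeginPlay it picks a sprite at random from its Sprites array.
; A DoOnce limits hit handling to the first collision; if that hit component is tagged "Sides", it finds the AudioManager in the level and calls SideHit.
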(event EventBeginPlay
  (bind _sprites (Variables|Default|GetSprites))
  (Rendering|Components|Sprite|SetSprite (Variables|Default|GetPaperSprite) (Utilities|Array|Get(acopy) _sprites (Math|Random|RandomInteger (Utilities|Array|Length _sprites)))))

(event Collision|EventHit
  (params (MyComp :type Primitive%20Component%20Object%20Reference) (Other :type Actor%20Object%20Reference) (OtherComp :type Primitive%20Component%20Object%20Reference) (bSelfMoved :type Boolean) (HitLocation :type Vector :default "0, 0, 0") (HitNormal :type Vector :default "0, 0, 0") (NormalImpulse :type Vector :default "0, 0, 0") (Hit :type Hit%20Result%20Structure%20%28by%20ref%29))
  (Utilities|FlowControl|DoOnce false
    (:Completed
      (if (Components|ComponentHasTag (.HitComponent (Collision|BreakHitResult Hit)) "Sides")
        (bind _outactors (Actor|GetAllActorsOfClass "/Game/Blueprints/Main/AudioManager.AudioManager_C"))
        (Default|SideHit _outactors)))))

(fn ConstructionScript)
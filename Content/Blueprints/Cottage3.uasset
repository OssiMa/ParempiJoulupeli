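; Cottage3 is a moving house actor that receives gifts dropped into it for a delivery game.
; Tick slides it along world X at MoveSpeed.
; Overlapping actors tagged Gift are destroyed and counted up to MaxGifts.
; Each accepted gift notifies the first GameManager found, calling FirstGiftDelivered while the house still NeedsGifts and MoreGifts afterwards.
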(event EventTick
  (params (DeltaSeconds :type Float%20%28single-precision%29))
  (bind _returnvalue (Transformation|GetActorTransform))
  (bind _returnvalue_2 (Math|Transform|TransformLocation _returnvalue "0, 0, 0"))
  (bind (_x _y _z) (Math|Vector|BreakVector _returnvalue_2))
  ;[1 1 1] House movement
  (Transformation|SetActorLocation (Math|Vector|MakeVector (+ (* DeltaSeconds (Variables|Default|GetmoveSpeed)) _x) _y _z) false false))

(event Collision|EventActorBeginOverlap
  (params (OtherActor :type Actor%20Object%20Reference))
  ;[1 1 1] Chimney
  (if (and (Actor|ActorHasTag OtherActor "Gift") (< (Variables|Default|GetgiftsInHouse) (Variables|Default|GetmaxGifts)))
    (Actor|DestroyActor OtherActor)
    (Variables|Default|SetgiftsInHouse (+ (Variables|Default|GetgiftsInHouse) 1))
    (bind _outactors (Actor|GetAllActorsOfClass "/Game/Blueprints/Main/GameManager.GameManager_C"))
    (if (Variables|Default|GetneedsGifts)
      (Default|FirstGiftDelivered (Utilities|Array|Get(acopy) _outactors))
      (Variables|Default|SetneedsGifts false)
      (else
        (Default|MoreGifts (Utilities|Array|Get(acopy) _outactors))))))

(fn ConstructionScript)
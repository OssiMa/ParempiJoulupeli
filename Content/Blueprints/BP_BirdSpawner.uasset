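; BP_BirdSpawner is a spawner that keeps producing BP_Bird actors from a left or right spawn point.
; From BeginPlay, SetSpawn picks a side at random, then re-arms a one-shot timer on itself with a short random delay.
; Left spawns set FacingLeft to true after spawning and print debug strings.
; Right spawns leave FacingLeft at its default, as the node setting it false is unconnected.
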(event Custom|LeftSideSpawn
  (Development|PrintString "Hello")
  (bind _returnvalue (Game|SpawnActorfromClass "/Game/Blueprints/BP_Bird.BP_Bird_C" (Math|Conversions|ToTransform(Vector) (Variables|Default|GetLeft%20Spawn)) "Undefined" 0 0))
  (bind _output_get (Variables|/Game/Blueprints/BP_Bird.BP_Bird_C|SetFacingLeft _returnvalue true))
  (Development|PrintString (Utilities|String|ToString(Boolean) _output_get)))

(event Custom|Set%20Spawn
  (if (Math|Random|RandomBool)
    (CallFunction|LeftSideSpawn)
    (else
      (CallFunction|RightSideSpawn)))
  (Utilities|Time|SetTimerbyEvent (delegate Custom|Set%20Spawn) (Math|Random|RandomFloatinRange 1.0 2.0)))

(event Custom|RightSideSpawn
  (bind _returnvalue (Game|SpawnActorfromClass "/Game/Blueprints/BP_Bird.BP_Bird_C" (Math|Conversions|ToTransform(Vector) (Variables|Default|GetRight%20Spawn)) "Undefined" 0 0)))

(event EventBeginPlay
  (CallFunction|SetSpawn))

(fn ConstructionScript)
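; BP_Bird is a bird actor that flies in a straight line until hit and removes itself after a fixed lifespan.
; Each Tick moves it along world X by MoveSpeed scaled by delta time, without sweeping for collisions.
; The Hit event fires once, setting IsHit to stop that movement and enabling physics and gravity on the Bird component so it can fall.
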(event EventTick
  (params (DeltaSeconds :type Float%20%28single-precision%29))
  (bind _returnvalue (Transformation|GetActorTransform))
  (bind _returnvalue_2 (Math|Transform|TransformLocation _returnvalue "0, 0, 0"))
  (bind (_x _y _z) (Math|Vector|BreakVector _returnvalue_2))
  ;[1 1 1] Bird movement
  (if (not (Variables|Default|GetIsHit))
    (Transformation|SetActorLocation (Math|Vector|MakeVector (+ (* DeltaSeconds (Variables|Default|GetMove%20Speed)) _x) _y _z) false false)))

(event Collision|EventHit
  (params (MyComp :type Primitive%20Component%20Object%20Reference) (Other :type Actor%20Object%20Reference) (OtherComp :type Primitive%20Component%20Object%20Reference) (bSelfMoved :type Boolean) (HitLocation :type Vector :default "0, 0, 0") (HitNormal :type Vector :default "0, 0, 0") (NormalImpulse :type Vector :default "0, 0, 0") (Hit :type Hit%20Result%20Structure%20%28by%20ref%29))
  (bind _bird (Variables|Default|GetBird))
  ;[1 1 1] On hit
  (if (not (Variables|Default|GetIsHit))
    (Physics|SetSimulatePhysics _bird true)
    (Physics|SetEnableGravity _bird true)
    (Variables|Default|SetIsHit true)))

(event EventBeginPlay
  ;[1 1 1] Set lifespan
  (Actor|SetLifeSpan 1e+01))

(fn ConstructionScript)
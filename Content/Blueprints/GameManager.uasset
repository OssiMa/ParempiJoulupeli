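; GameManager tracks lives, score and delivered presents for a gift-delivery game.
; A missed gift prints a message and costs a life, and running out pauses the game and shows the game over widget.
; The delivery events count each present and add points, with the first gift worth more than later ones.
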(event Custom|MissGift
  ;[1 1 1] Losing lives
  (Development|PrintString "Oh no you dropped a gift :(")
  (Variables|Default|SetLives (+ (Variables|Default|GetLives) -1))
  (if (<= (Variables|Default|GetLives) 0)
    (Game|SetGamePaused true)
    (bind _returnvalue (UserInterface|CreateWidget "/Game/Blueprints/MainGameHUD/BP_GameOverWidget.BP_GameOverWidget_C"))
    (UserInterface|Viewport|AddtoViewport _returnvalue 0)))

(event Custom|FirstGiftDelivered
  ;[1 1 1] Scoring
  (Variables|Default|SetPresentsDelivered (+ (Variables|Default|GetPresentsDelivered) 1))
  (Variables|Default|SetScore (+ (Variables|Default|GetScore) 500)))

(event Custom|MoreGifts
  ;[1 1 1] Scoring
  (Variables|Default|SetPresentsDelivered (+ (Variables|Default|GetPresentsDelivered) 1))
  (Variables|Default|SetScore (+ (Variables|Default|GetScore) 100)))

(fn ConstructionScript)
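; Long chimney actor that scrolls along X each tick and receives gifts for its owning BP_House.
; When a Gift-tagged actor overlaps and the house is below its gift limit, it removes the gift from BP_Santa's spawned list and notifies the house.
; An accepted gift also triggers a one-shot smoke puff and a timeline-driven squash-and-stretch of the sprite, guarded against restarting mid-animation.
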(event OnFinishedPlaying(Smoke)
  ;[1 1 1] Puff of smoke
  (Rendering|SetVisibility (Variables|Default|GetSmoke) false false))

(event Custom|PlayEffect
  (bind _smoke (Variables|Default|GetSmoke))
  ;[1 1 1] Puff of smoke
  (Rendering|SetVisibility _smoke true false)
  (Components|Timeline|PlayfromStart _smoke))

(event EventTick
  (params (DeltaSeconds :type Float%20%28single-precision%29))
  (bind _returnvalue (Transformation|GetActorTransform))
  (bind _returnvalue_2 (Math|Transform|TransformLocation _returnvalue "0, 0, 0"))
  (bind (_x _y _z) (Math|Vector|BreakVector _returnvalue_2))
  ;[1 1 1] House movement
  (Transformation|SetActorLocation (Math|Vector|MakeVector (+ (* DeltaSeconds (Variables|Default|GetmoveSpeed)) _x) _y _z) false false))

(event EventBeginPlay
  (bind _smoke (Variables|Default|GetSmoke))
  ;[1 1 1] Puff of smoke
  (Rendering|SetVisibility _smoke false false)
  (Components|Timeline|SetLooping _smoke false))

(event Collision|EventActorBeginOverlap
  (params (OtherActor :type Actor%20Object%20Reference))
  (bind _papersprite (Variables|Default|GetPaperSprite))
  ;[1 1 1] Gifts going in
  (if (Actor|ActorHasTag OtherActor "Gift")
    (bind _asbp_house (Utilities|Casting|CastToBP_House (Components|GetOwner)))
    (Math|Integer|CompareInt (Variables|/Game/Blueprints/Main/BP_House.BP_House_C|GetgiftsInHouse _asbp_house) (Variables|/Game/Blueprints/Main/BP_House.BP_House_C|GetmaxGifts _asbp_house)
      (:<
        (Variables|/Game/Blueprints/Main/BP_House.BP_House_C|SetgiftReference _asbp_house OtherActor)
        (bind _outactors (Actor|GetAllActorsOfClass "/Game/Blueprints/BP_Santa.BP_Santa_C"))
        (CallFunction|PlayEffect)
        (Utilities|Array|RemoveIndex (Variables|/Game/Blueprints/BP_Santa.BP_Santa_C|GetSpawnedGifts (Utilities|Array|Get(acopy) _outactors)) (Utilities|Array|FindItem (Variables|/Game/Blueprints/BP_Santa.BP_Santa_C|GetSpawnedGifts (Utilities|Array|Get(acopy) _outactors)) OtherActor))
        (Default|GiftinChimney _asbp_house)
        ;[1 1 1] Animation
        (if (not (Variables|Default|GetanimPlaying))
          (Variables|Default|SetanimPlaying true)
          (Variables|Default|SetNewVar_0 (.Scale (Math|Transform|BreakTransform (Transformation|GetWorldTransform _papersprite))))
          (bind (_direction _x_stretch _z_squash) (Timeline|Timeline_0 PlayFromStart)
            (:Update
              (Transformation|SetWorldScale3D _papersprite (Math|Vector|MakeVector (+ (.X (Math|Vector|BreakVector (Variables|Default|GetNewVar_0))) _x_stretch) 0.0 (+ (.Z (Math|Vector|BreakVector (Variables|Default|GetNewVar_0))) _z_squash))))
            (:Finished
              (Variables|Default|SetanimPlaying false))))))))

(fn ConstructionScript)
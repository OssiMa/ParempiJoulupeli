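; BP_Chimney is a moving chimney target that detects gifts dropping into it and reports them to its house.
; Tick shifts it along world X at MoveSpeed, scaled by delta time and without sweeping.
; An overlap that passes the "Gift" tag check stores the gift on the owning BP_House, updates the first BP_Santa's SpawnedGifts list by removal, then calls the house's GiftInChimney.
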(event EventTick
  (params (DeltaSeconds :type Float%20%28single-precision%29))
  (bind _returnvalue (Transformation|GetActorTransform))
  (bind _returnvalue_2 (Math|Transform|TransformLocation _returnvalue "0, 0, 0"))
  (bind (_x _y _z) (Math|Vector|BreakVector _returnvalue_2))
  ;[1 1 1] House movement
  (Transformation|SetActorLocation (Math|Vector|MakeVector (+ (* DeltaSeconds (Variables|Default|GetmoveSpeed)) _x) _y _z) false false))

(event Collision|EventActorBeginOverlap
  (params (OtherActor :type Actor%20Object%20Reference))
  ;[1 1 1] Gifts going in
  (if (Actor|ActorHasTag "Gift")
    (bind _asbp_house (Utilities|Casting|CastToBP_House (Components|GetOwner)))
    (Variables|/Game/Blueprints/Main/BP_House.BP_House_C|SetgiftReference _asbp_house OtherActor)
    (bind _outactors (Actor|GetAllActorsOfClass "/Game/Blueprints/BP_Santa.BP_Santa_C"))
    (Utilities|Array|RemoveIndex (Variables|/Game/Blueprints/BP_Santa.BP_Santa_C|GetSpawnedGifts (Utilities|Array|Get(acopy) _outactors)) (Utilities|Array|FindItem (Variables|/Game/Blueprints/BP_Santa.BP_Santa_C|GetSpawnedGifts (Utilities|Array|Get(acopy) _outactors)) 0))
    (Default|GiftinChimney _asbp_house)))

(fn ConstructionScript)
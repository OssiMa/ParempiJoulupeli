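; BP_Chimney_Busted is a chimney actor, by its name a broken variant, that scrolls continuously along the world X axis.
; Each Tick it reads SpeedModifier from GlobalInstance, scales it negatively and adds it to its own MoveSpeed.
; It applies that speed times delta seconds to X through a non-swept SetActorLocation, keeping Y and Z unchanged.
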(event EventTick
  (params (DeltaSeconds :type Float%20%28single-precision%29))
  (bind _returnvalue (Transformation|GetActorTransform))
  (bind _returnvalue_2 (Math|Transform|TransformLocation _returnvalue "0, 0, 0"))
  (bind (_x _y _z) (Math|Vector|BreakVector _returnvalue_2))
  ;[1 1 1] House movement
  (bind _asglobal_instance (Utilities|Casting|CastToGlobalInstance (Game|GetGameInstance)))
  (Transformation|SetActorLocation (Math|Vector|MakeVector (+ (* DeltaSeconds (+ (* (Variables|/Game/Blueprints/GlobalInstance.GlobalInstance_C|GetSpeedModifier _asglobal_instance) -5.0) (Variables|Default|GetmoveSpeed))) _x) _y _z) false false))

(fn ConstructionScript)
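; Giant chimney actor that scrolls along world X at MoveSpeed and serves as a drop target for gifts.
; Each overlapping actor tagged Gift decrements GiftsNeeded while the chimney is Empty.
; While gifts are still needed, it destroys the gift and reports a delivery to the GameManager.
; The final gift is not destroyed; it clears the owning BP_House's NeedsGifts, calls LastGift and closes the chimney.
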(event EventTick
  (params (DeltaSeconds :type Float%20%28single-precision%29))
  (bind _returnvalue (Transformation|GetActorTransform))
  (bind _returnvalue_2 (Math|Transform|TransformLocation _returnvalue "0, 0, 0"))
  (bind (_x _y _z) (Math|Vector|BreakVector _returnvalue_2))
  ;[1 1 1] House movement
  (Transformation|SetActorLocation (Math|Vector|MakeVector (+ (* DeltaSeconds (Variables|Default|GetmoveSpeed)) _x) _y _z) false false))

(event Collision|EventActorBeginOverlap
  (params (OtherActor :type Actor%20Object%20Reference))
  ;[1 1 1] Gifts going in
  (if (and (Actor|ActorHasTag OtherActor "Gift") (Variables|Default|Getempty))
    (Variables|Default|SetgiftsNeeded (+ (Variables|Default|GetgiftsNeeded) -1))
    (Math|Integer|CompareInt (Variables|Default|GetgiftsNeeded)
      (:>
        (Actor|DestroyActor OtherActor)
        (bind _outactors (Actor|GetAllActorsOfClass "/Game/Blueprints/Main/GameManager.GameManager_C"))
        (Default|GiftDelivered _outactors 1))
      (:==
        (bind _asbp_house (Utilities|Casting|CastToBP_House (Components|GetOwner) :!label _label))
        (Variables|/Game/Blueprints/Main/BP_House.BP_House_C|SetneedsGifts _asbp_house false)
        (bind _outactors_2 (Actor|GetAllActorsOfClass "/Game/Blueprints/Main/GameManager.GameManager_C"))
        (Default|LastGift _outactors_2)
        (Variables|Default|Setempty false))
      (:<
        (goto _label)))))

(fn ConstructionScript)
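; Chimney opening actor with a cycling hatch that catches gifts for its house.
; Tick slides it along X at MoveSpeed and swings HatchRotator between two pitch limits, using the Open flag and Delays to pause before reversing.
; On overlap with a "Gift"-tagged actor, it passes the gift to its owning BP_House, removes it from BP_Santa's SpawnedGifts and calls GiftInChimney.
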(event EventTick
  (params (DeltaSeconds :type Float%20%28single-precision%29))
  (bind _returnvalue (Transformation|GetActorTransform))
  (bind _hatchrotator (Variables|Default|GethatchRotator))
  (bind _returnvalue_2 (Math|Transform|TransformLocation _returnvalue "0, 0, 0"))
  (bind _relativerotation (Variables|/Script/Engine.SceneComponent|GetRelativeRotation _hatchrotator))
  (bind (_x _y _z) (Math|Vector|BreakVector _returnvalue_2))
  (bind _pitch (Math|Rotator|BreakRotator _relativerotation))
  ;[1 1 1] House movement
  (Transformation|SetActorLocation (Math|Vector|MakeVector (+ (* DeltaSeconds (Variables|Default|GetmoveSpeed)) _x) _y _z) false false)
  ;[1 1 1] Rotator
  (if (Variables|Default|Getopen)
    (Math|Float|CompareFloat _pitch 0.0
      (:>
        (Utilities|FlowControl|Delay 0.2 :!label _label)
        (Variables|Default|Setopen false))
      (:==
        (goto _label))
      (:<
        (Transformation|AddRelativeRotation _hatchrotator (Math|Rotator|MakeRotator 0.0 (* 45.0 (Utilities|Time|GetWorldDeltaSeconds)) 0.0) false false)))
    (else
      (Math|Float|CompareFloat _pitch -88.0
        (:>
          (Transformation|AddRelativeRotation _hatchrotator (Math|Rotator|MakeRotator 0.0 (* -9e+01 (Utilities|Time|GetWorldDeltaSeconds)) 0.0) false false))
        (:==
          (Utilities|FlowControl|Delay 2.0 :!label _label_2)
          (Variables|Default|Setopen true))
        (:<
          (goto _label_2))))))

(event Collision|EventActorBeginOverlap
  (params (OtherActor :type Actor%20Object%20Reference))
  ;[1 1 1] Gifts going in
  (if (Actor|ActorHasTag OtherActor "Gift")
    (bind _asbp_house (Utilities|Casting|CastToBP_House (Components|GetOwner)))
    (Variables|/Game/Blueprints/Main/BP_House.BP_House_C|SetgiftReference _asbp_house OtherActor)
    (bind _outactors (Actor|GetAllActorsOfClass "/Game/Blueprints/BP_Santa.BP_Santa_C"))
    (Utilities|Array|RemoveIndex (Variables|/Game/Blueprints/BP_Santa.BP_Santa_C|GetSpawnedGifts (Utilities|Array|Get(acopy) _outactors)) (Utilities|Array|FindItem (Variables|/Game/Blueprints/BP_Santa.BP_Santa_C|GetSpawnedGifts (Utilities|Array|Get(acopy) _outactors)) OtherActor))
    (Default|GiftinChimney _asbp_house)))

(fn ConstructionScript)
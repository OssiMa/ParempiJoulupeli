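; BP_Chimney_Cover is a house chimney with a removable top that receives gifts as it scrolls along X.
; Tick offsets its location by MoveSpeed scaled by delta time.
; Any overlapping actor is passed to the owning BP_House as GiftReference, then GiftInChimney is called.
; A hit on either of the two cover Paper2D sprites destroys both after a short delay.
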(event EventTick
  (params (DeltaSeconds :type Float%20%28single-precision%29))
  (bind _returnvalue (Transformation|GetActorTransform))
  (bind _returnvalue_2 (Math|Transform|TransformLocation _returnvalue "0, 0, 0"))
  (bind (_x _y _z) (Math|Vector|BreakVector _returnvalue_2))
  ;[1 1 1] House movement
  (Transformation|SetActorLocation (Math|Vector|MakeVector (+ (* DeltaSeconds (Variables|Default|GetmoveSpeed)) _x) _y _z) false false))

(event Collision|EventHit
  (params (MyComp :type Primitive%20Component%20Object%20Reference) (Other :type Actor%20Object%20Reference) (OtherComp :type Primitive%20Component%20Object%20Reference) (bSelfMoved :type Boolean) (HitLocation :type Vector :default "0, 0, 0") (HitNormal :type Vector :default "0, 0, 0") (NormalImpulse :type Vector :default "0, 0, 0") (Hit :type Hit%20Result%20Structure%20%28by%20ref%29))
  ;[1 1 1] Removable top
  (if (or (== MyComp (Variables|Default|GetPaperSprite2)) (== MyComp (Variables|Default|GetPaperSprite1)))
    (Utilities|FlowControl|Delay 0.2)
    (Components|DestroyComponent (Variables|Default|GetPaperSprite1))
    (Components|DestroyComponent (Variables|Default|GetPaperSprite2))))

(event Collision|EventActorBeginOverlap
  (params (OtherActor :type Actor%20Object%20Reference))
  ;[1 1 1] Gifts going in
  (bind _asbp_house (Utilities|Casting|CastToBP_House (Components|GetOwner)))
  (Variables|/Game/Blueprints/Main/BP_House.BP_House_C|SetgiftReference _asbp_house OtherActor)
  (Default|GiftinChimney _asbp_house))

(fn ConstructionScript)
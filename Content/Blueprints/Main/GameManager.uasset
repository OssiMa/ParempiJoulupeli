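; GameManager tracks lives, score and delivered presents for a gift-delivery game, and runs the game-over flow.
; Missed gifts cost lives, while deliveries add multiplied points or a last-gift bonus and notify the first BP_HouseSpawner.
; Game over pauses play, saves any new highscore to BP_SaveData in the "Calendar" slot, and shows BP_GameOverWidget.
; The UnlockManager scoring call after the final miss has no target connected.
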(event Custom|MissGift
  ;[1 1 1] Losing lives
  (Variables|Default|SetLives (+ (Variables|Default|GetLives) -1))
  (if (<= (Variables|Default|GetLives) 0)
    (CallFunction|GameOver)
    (bind _outactors (Actor|GetAllActorsOfClass 0))
    (bind _output_get (Variables|Default|SetUnlockManager 0 0))
    (CallFunction|ScoreEtc _output_get)))

(event Custom|GiftDelivered
  (params (ScoreMultiplier :type Integer))
  ;[1 1 1] Scoring
  (Variables|Default|SetPresentsDelivered (+ (Variables|Default|GetPresentsDelivered) 1))
  (Variables|Default|SetScore (+ (Variables|Default|GetScore) (* 50 ScoreMultiplier)))
  (bind _outactors (Actor|GetAllActorsOfClass "/Game/Blueprints/BP_HouseSpawner.BP_HouseSpawner_C"))
  (bind _output_get (Variables|Default|SetTargetBlueprint (Utilities|Array|Get(acopy) _outactors)))
  (Default|SetPresentsDelivered _output_get))

(event Custom|GameOver
  (bind _score (Variables|Default|GetScore))
  ;[1 1 1] Ends the game, calculates highscore and displays gameover-screen
  (Game|SetGamePaused true)
  (bind _returnvalue (SaveGame|DoesSaveGameExist "Calendar"))
  (if _returnvalue
    (bind _returnvalue_2 (SaveGame|LoadGamefromSlot "Calendar"))
    (Variables|Default|SetSaveInstance _returnvalue_2)
    (else
      (bind _returnvalue_3 (SaveGame|CreateSaveGameObject "/Game/Blueprints/Calendar/SavingAndWidgets/BP_SaveData.BP_SaveData_C"))
      (Variables|Default|SetSaveInstance _returnvalue_3)))
  (bind _asbp_save_data (Utilities|Casting|CastToBP_SaveData (Variables|Default|GetSaveInstance)))
  (Math|Integer|CompareInt (Variables|/Game/Blueprints/Calendar/SavingAndWidgets/BP_SaveData.BP_SaveData_C|GetHighscore _asbp_save_data) _score
    (:>
      _)
    (:==
      _)
    (:<
      (Variables|/Game/Blueprints/Calendar/SavingAndWidgets/BP_SaveData.BP_SaveData_C|SetHighscore _asbp_save_data _score)
      (SaveGame|SaveGametoSlot _asbp_save_data "Calendar")))
  (Viewport|RemoveAllWidgets)
  (bind _returnvalue_4 (UserInterface|CreateWidget "/Game/Blueprints/MainGameHUD/BP_GameOverWidget.BP_GameOverWidget_C"))
  (UserInterface|Viewport|AddtoViewport _returnvalue_4 0))

(event Custom|LastGift
  ;[1 1 1] Scoring
  (Variables|Default|SetScore (+ (Variables|Default|GetScore) 500))
  (Variables|Default|SetPresentsDelivered (+ (Variables|Default|GetPresentsDelivered) 1))
  (bind _outactors (Actor|GetAllActorsOfClass "/Game/Blueprints/BP_HouseSpawner.BP_HouseSpawner_C"))
  (bind _output_get (Variables|Default|SetTargetBlueprint (Utilities|Array|Get(acopy) _outactors)))
  (Default|SetPresentsDelivered _output_get))

(fn ConstructionScript)
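; Manager actor that tracks calendar day unlocks from the player's score and persists completed days.
; BeginPlay caches the GlobalInstance's completed days and last visited month.
; ScoreEtc runs CompareDays, then on reaching the unlock threshold resets the saved score and writes completed days to the "Calendar" BP_SaveData slot, creating it if missing.
; SetUnlockedDay adds a day count to the GlobalInstance's completed days, without saving.
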(event Custom|ScoreEtc
  (Variables|Default|SetpresentScore (Variables|/Game/Blueprints/GlobalInstance.GlobalInstance_C|GetSavedScore (stale EventBeginPlay _asglobal_instance)))
  (Class|UnlockManager|CompareDays)
  (if (>= (Variables|/Game/Blueprints/GlobalInstance.GlobalInstance_C|GetSavedScore (stale EventBeginPlay _asglobal_instance)) (Variables|Default|GetscoreForUnlocking))
    (Variables|/Game/Blueprints/GlobalInstance.GlobalInstance_C|SetSavedScore (stale EventBeginPlay _asglobal_instance) 0)
    ;[1 1 1] Save Unlock
    (bind _returnvalue (SaveGame|DoesSaveGameExist "Calendar"))
    (if _returnvalue
      (bind _returnvalue_2 (SaveGame|LoadGamefromSlot "Calendar"))
      (bind _asbp_save_data (Utilities|Casting|CastToBP_SaveData _returnvalue_2))
      (Variables|Default|SetSaveRef _asbp_save_data)
      (else
        (bind _returnvalue_3 (SaveGame|CreateSaveGameObject "/Game/Blueprints/Calendar/SavingAndWidgets/BP_SaveData.BP_SaveData_C"))
        (Variables|Default|SetSaveRef _returnvalue_3)))
    (bind _asglobal_instance (Utilities|Casting|CastToGlobalInstance (Game|GetGameInstance)))
    (Variables|/Game/Blueprints/Calendar/SavingAndWidgets/BP_SaveData.BP_SaveData_C|SetCompletedDays (Variables|Default|GetSaveRef) (Variables|/Game/Blueprints/GlobalInstance.GlobalInstance_C|GetCompletedDays _asglobal_instance))
    (SaveGame|SaveGametoSlot (Variables|Default|GetSaveRef) "Calendar")))

(event EventBeginPlay
  (bind _asglobal_instance (Utilities|Casting|CastToGlobalInstance (Game|GetGameInstance)))
  (Variables|Default|SetlastUnlockedDay (Variables|/Game/Blueprints/GlobalInstance.GlobalInstance_C|GetCompletedDays _asglobal_instance))
  (Variables|Default|SetlastSavedMonth (Variables|/Game/Blueprints/GlobalInstance.GlobalInstance_C|GetLastVisitedMonth _asglobal_instance)))

(event EventSetUnlockedDay
  (params (dayCount :type Integer%20%28by%20ref%29))
  (bind _asglobal_instance (Utilities|Casting|CastToGlobalInstance (Game|GetGameInstance)))
  (Variables|/Game/Blueprints/GlobalInstance.GlobalInstance_C|SetCompletedDays _asglobal_instance (+ (Variables|/Game/Blueprints/GlobalInstance.GlobalInstance_C|GetCompletedDays _asglobal_instance) dayCount)))

(fn ConstructionScript)
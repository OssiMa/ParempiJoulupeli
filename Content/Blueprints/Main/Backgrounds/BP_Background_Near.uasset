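; BP_Background_Near is the near background layer, a plane that shows a scrolling backdrop for the current map.
; After a brief BeginPlay delay, it reads CurrentMap from the GlobalInstance and creates a dynamic material from the matching NearBackgrounds entry.
; Tick drives that material's U Offset from game time divided by OffsetSpeed, scrolling through the material rather than moving the actor.
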(event EventBeginPlay
  ;[1 1 1] Chooses the correct background
  (Utilities|FlowControl|Delay 0.01)
  (bind _asglobal_instance (Utilities|Casting|CastToGlobalInstance (Game|GetGameInstance)))
  (bind _returnvalue (Rendering|Material|CreateDynamicMaterialInstance (Variables|Default|GetPlane) 0 (Utilities|Array|Get(acopy) (Variables|Default|GetNearBackgrounds) (Variables|/Game/Blueprints/GlobalInstance.GlobalInstance_C|GetCurrentMap _asglobal_instance)) "None" :!class /Script/Engine.PrimitiveComponent)))

(event EventTick
  (params (DeltaSeconds :type Float%20%28single-precision%29))
  ;[1 1 1] Movement
  (Rendering|Material|SetScalarParameterValue (stale EventBeginPlay _returnvalue) "U Offset" (/ (Utilities|Time|GetGameTimeinSeconds) (Variables|Default|GetOffsetSpeed)) :!class /Script/Engine.MaterialInstanceDynamic))

(fn ConstructionScript)
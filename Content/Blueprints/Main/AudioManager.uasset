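; Central audio manager that starts the music on BeginPlay and exposes events for the game's sound effects.
; Throw and SideHit play a random pick from their sets of throw and thump sounds to vary repeats.
; Delivery, WindSound and Filled each play a dedicated sound.
; MinorEffect swaps the passed-in sound onto one shared MinorEffects component and plays it, so minor sounds share a single player.
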(event Custom|Throw
  (bind _throw3 (Variables|Default|GetThrow3))
  (bind _throw4 (Variables|Default|GetThrow4))
  (bind _throw5 (Variables|Default|GetThrow5))
  (bind _throw1 (Variables|Default|GetThrow1))
  (bind _throw2 (Variables|Default|GetThrow2))
  (bind _array (Utilities|Array|MakeArray _throw1 _throw2 _throw3 _throw4 _throw5))
  ;[1 1 1] Throw
  (Audio|Components|Audio|Play (Utilities|Array|Get(acopy) _array (Math|Random|RandomIntegerinRange 0 (- (Utilities|Array|Length _array) 1))) 0.0))

(event Custom|Delivery
  ;[1 1 1] Delivery
  (Audio|Components|Audio|Play (Variables|Default|GetDelivered) 0.0))

(event Custom|MinorEffect
  (params (SoundToPlay :type Sound%20Cue%20Object%20Reference))
  (bind _minoreffects (Variables|Default|GetMinorEffects))
  ;[1 1 1] Play minor sound effects
  (Audio|Components|Audio|SetSound _minoreffects SoundToPlay)
  (Audio|Components|Audio|Play _minoreffects 0.0))

(event Custom|SideHit
  (bind _thump1 (Variables|Default|GetThump1))
  (bind _thump2 (Variables|Default|GetThump2))
  (bind _thump3 (Variables|Default|GetThump3))
  (bind _thump4 (Variables|Default|GetThump4))
  (bind _thump5 (Variables|Default|GetThump5))
  (bind _thump6 (Variables|Default|GetThump6))
  (bind _thump7 (Variables|Default|GetThump7))
  (bind _array (Utilities|Array|MakeArray _thump1 _thump2 _thump3 _thump4 _thump5 _thump6 _thump7))
  ;[1 1 1] SideHit
  (Audio|Components|Audio|Play (Utilities|Array|Get(acopy) _array (Math|Random|RandomIntegerinRange 0 (- (Utilities|Array|Length _array) 1))) 0.0))

(event Custom|WindSound
  (Audio|Components|Audio|Play (Variables|Default|GetWind) 0.0))

(event Custom|Filled
  (Audio|Components|Audio|Play (Variables|Default|GetFilledSound) 0.0))

(event EventBeginPlay
  (Audio|Components|Audio|Play (Variables|Default|GetMusic) 0.0))

(fn ConstructionScript)
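; Game manager for a present-delivery game that tracks score, lives and presents delivered.
; A first delivery awards a large bonus, while further gifts award less and also increment the target Blueprint's present value.
; Misses cost a life, and running out triggers GameOver.
; GameOver pauses the game, saves any new highscore to the existing "Calendar" save slot, and replaces all widgets with the game-over screen.
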(event Custom|MissGift
  ;[1 1 1] Losing lives
  (Variables|Default|SetLives (+ (Variables|Default|GetLives) -1))
  (if (<= (Variables|Default|GetLives) 0)
    (CallFunction|GameOver)))

(event Custom|FirstGiftDelivered
  ;[1 1 1] Scoring
  (Variables|Default|SetPresentsDelivered_0 (+ (Variables|Default|GetPresentsDelivered_0) 1))
  (Variables|Default|SetScore (+ (Variables|Default|GetScore) 500)))

(event Custom|MoreGifts
  ;[1 1 1] Scoring
  (Variables|Default|SetPresentsDelivered_0 (+ (Variables|Default|GetPresentsDelivered_0) 1))
  (Variables|Default|SetScore (+ (Variables|Default|GetScore) 100))
  (Variables|/Game/Blueprints/BP_HouseSpawner.BP_HouseSpawner_C|SetPresentsValue (Variables|Default|GetTargetBlueprint) (+ (Variables|/Game/Blueprints/BP_HouseSpawner.BP_HouseSpawner_C|GetPresentsValue (Variables|Default|GetTargetBlueprint)) 1)))

(event Custom|GameOver
  (bind _score (Variables|Default|GetScore))
  ;[1 1 1] Ends the game, calculates highscore and displays gameover-screen
  (Game|SetGamePaused true)
  (bind _returnvalue (SaveGame|LoadGamefromSlot "Calendar"))
  (bind _asbp_save_data (Utilities|Casting|CastToBP_SaveData _returnvalue))
  (Math|Integer|CompareInt (Variables|/Game/Blueprints/Calendar/BP_SaveData.BP_SaveData_C|GetHighscore _asbp_save_data) _score
    (:>
      _)
    (:==
      _)
    (:<
      (Variables|/Game/Blueprints/Calendar/BP_SaveData.BP_SaveData_C|SetHighscore _asbp_save_data _score)
      (SaveGame|SaveGametoSlot _asbp_save_data "Calendar")))
  (Viewport|RemoveAllWidgets)
  (bind _returnvalue_2 (UserInterface|CreateWidget "/Game/Blueprints/MainGameHUD/BP_GameOverWidget.BP_GameOverWidget_C"))
  (UserInterface|Viewport|AddtoViewport _returnvalue_2 0))

(fn ConstructionScript)
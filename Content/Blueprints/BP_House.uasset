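; BP_House is a scrolling Paper2D house that accepts gifts through its chimney.
; BeginPlay sets a random sprite from a per-map array (DefaultSprites for all three maps) and spawns a random chimney at a second sprite's location.
; Tick moves the house along X at MoveSpeed.
; GiftInChimney destroys tagged gifts up to a per-house limit and notifies GameManager, distinguishing the first needed gift from extras.
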(event Custom|Randomizer
  ;[1 1 1] Choose random chimney
  (Variables|Default|SetchosenChimney (Utilities|Array|Get(acopy) (Variables|Default|GetchimneyArray) (Math|Random|RandomIntegerinRange 0 (+ (Utilities|Array|Length (Variables|Default|GetchimneyArray)) -1)))))

(event Custom|GiftInChimney
  (bind _giftreference (Variables|Default|GetgiftReference))
  ;[1 1 1] Chimney
  (if (and (Actor|ActorHasTag _giftreference "Gift") (< (Variables|Default|GetgiftsInHouse) (Variables|Default|GetmaxGifts)))
    (Actor|DestroyActor _giftreference)
    (Variables|Default|SetgiftsInHouse (+ (Variables|Default|GetgiftsInHouse) 1))
    (bind _outactors (Actor|GetAllActorsOfClass "/Game/Blueprints/Main/GameManager.GameManager_C"))
    (if (Variables|Default|GetneedsGifts)
      (Default|FirstGiftDelivered (Utilities|Array|Get(acopy) _outactors))
      (Variables|Default|SetneedsGifts false)
      (else
        (Default|MoreGifts (Utilities|Array|Get(acopy) _outactors))))))

(event EventTick
  (params (DeltaSeconds :type Float%20%28single-precision%29))
  (bind _returnvalue (Transformation|GetActorTransform))
  (bind _returnvalue_2 (Math|Transform|TransformLocation _returnvalue "0, 0, 0"))
  (bind (_x _y _z) (Math|Vector|BreakVector _returnvalue_2))
  ;[1 1 1] House movement
  (Transformation|SetActorLocation (Math|Vector|MakeVector (+ (* DeltaSeconds (Variables|Default|GetmoveSpeed)) _x) _y _z) false false))

(event EventBeginPlay
  ;[1 1 1] Sprite Randomizer
  (bind _asglobal_instance (Utilities|Casting|CastToGlobalInstance (Game|GetGameInstance)))
  (switch int (Variables|/Game/Blueprints/GlobalInstance.GlobalInstance_C|GetCurrentMap _asglobal_instance)
    (:0
      (Variables|Default|SetSpriteArrayRef (Variables|Default|GetdefaultSprites)))
    (:1
      (Variables|Default|SetSpriteArrayRef (Variables|Default|GetdefaultSprites)))
    (:2
      (Variables|Default|SetSpriteArrayRef (Variables|Default|GetdefaultSprites))))
  (Rendering|Components|Sprite|SetSprite (Variables|Default|GetPaperSprite) (Utilities|Array|Get(acopy) (Variables|Default|GetSpriteArrayRef) (Math|Random|RandomIntegerinRange 0 (+ (Utilities|Array|Length (Variables|Default|GetSpriteArrayRef)) -1))))
  (CallFunction|Randomizer)
  (bind _returnvalue (Game|SpawnActorfromClass (Variables|Default|GetchosenChimney) (Math|Conversions|ToTransform(Vector) (Transformation|GetWorldLocation (Variables|Default|GetPaperSprite1))) "Undefined" self 0))
  (Variables|Default|SetchimneyRef _returnvalue))

(fn ConstructionScript)
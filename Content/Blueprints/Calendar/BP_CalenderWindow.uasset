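; Advent-calendar window actor that opens on touch to grant the player that day's unlock.
; Opening requires the day of month and GlobalInstance's CompletedDays to reach OpeningDay; month checks lead nowhere.
; Opening swaps the sprite, plays a puff leading to a popup, increments GlobalInstance unlocks or sets day-event flags, and saves through BP_SaveDataActor.
; Load restores opened state by finding itself in the saved window array.
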(event OnFinishedPlaying(PopupExplosion)
  (bind _popupexplosion (Variables|Default|GetPopupExplosion))
  ;[1 1 1] Puff
  (if (Rendering|IsVisible _popupexplosion)
    (Rendering|SetVisibility _popupexplosion false false)
    (bind _returnvalue (UserInterface|CreateWidget "/Game/Blueprints/Calendar/SavingAndWidgets/BP_CalenderPopup.BP_CalenderPopup_C" 0 (Variables|Default|GetAvailableUnlock) (Variables|Default|GetOpeningDay)))
    (UserInterface|Viewport|AddtoViewport _returnvalue 0)))

(event Custom|Activate%20event
  (params (Global%20instance :type Global%20Instance%20Object%20Reference))
  ;[1 1 1] Activate events
  (Variables|/Game/Blueprints/GlobalInstance.GlobalInstance_C|SetIncreaseHouseSpawns Global%20instance (Variables|Default|GetBusy%20day))
  (Variables|/Game/Blueprints/GlobalInstance.GlobalInstance_C|SetWindy Global%20instance (Variables|Default|GetWindy%20day))
  (Variables|/Game/Blueprints/GlobalInstance.GlobalInstance_C|SetSpawnBirds Global%20instance (Variables|Default|GetBirdy%20day)))

(event Custom|Unlock
  ;[1 1 1] Unlocking upgrades
  (bind _asglobal_instance (Utilities|Casting|CastToGlobalInstance (Game|GetGameInstance)))
  (switch string (Variables|Default|GetAvailableUnlock)
    (:Default
      (CallFunction|ActivateEvent _asglobal_instance))
    (:decoration
      (Variables|/Game/Blueprints/GlobalInstance.GlobalInstance_C|SetVisualUpgrades _asglobal_instance (+ (Variables|/Game/Blueprints/GlobalInstance.GlobalInstance_C|GetVisualUpgrades _asglobal_instance) 1)))
    (:present
      (Variables|/Game/Blueprints/GlobalInstance.GlobalInstance_C|SetPresentUnlocks _asglobal_instance (+ (Variables|/Game/Blueprints/GlobalInstance.GlobalInstance_C|GetPresentUnlocks _asglobal_instance) 1)))
    (:map%20and%20present
      (Variables|/Game/Blueprints/GlobalInstance.GlobalInstance_C|SetPresentUnlocks _asglobal_instance (+ (Variables|/Game/Blueprints/GlobalInstance.GlobalInstance_C|GetPresentUnlocks _asglobal_instance) 1))
      (Variables|/Game/Blueprints/GlobalInstance.GlobalInstance_C|SetMapsUnlocked _asglobal_instance (+ (Variables|/Game/Blueprints/GlobalInstance.GlobalInstance_C|GetMapsUnlocked _asglobal_instance) 1) :!label _label)
      (Variables|/Game/Blueprints/GlobalInstance.GlobalInstance_C|SetCurrentMap _asglobal_instance (Variables|/Game/Blueprints/GlobalInstance.GlobalInstance_C|GetMapsUnlocked _asglobal_instance)))
    (:chimney
      (Variables|/Game/Blueprints/GlobalInstance.GlobalInstance_C|SetChimneyUnlocks _asglobal_instance (+ (Variables|/Game/Blueprints/GlobalInstance.GlobalInstance_C|GetChimneyUnlocks _asglobal_instance) 1)))
    (:map
      (goto _label))))

(event Custom|Set%20Status%20Opened
  ;[1 1 1] Opens the window
  (if (Variables|Default|GetOpened)
    ;[1 1 1] Opened Popup
    (if (not (Audio|Components|Audio|IsPlaying (Variables|Default|GetPopupExplosion)))
      (bind _returnvalue (UserInterface|CreateWidget "/Game/Blueprints/Calendar/SavingAndWidgets/BP_CalenderPopupOpened.BP_CalenderPopupOpened_C" 0 (Variables|Default|GetAvailableUnlock) (Variables|Default|GetOpeningDay) self))
      (UserInterface|Viewport|AddtoViewport _returnvalue 0)
      (Variables|/Game/Blueprints/GlobalInstance.GlobalInstance_C|SetPopupOpen (stale _asglobal_instance) true))
    (else
      ;[1 1 1] Is the day completed?
      (bind _asglobal_instance (Utilities|Casting|CastToGlobalInstance (Game|GetGameInstance)))
      (Math|Integer|CompareInt (Variables|Default|GetOpeningDay) (Variables|/Game/Blueprints/GlobalInstance.GlobalInstance_C|GetCompletedDays _asglobal_instance)
        (:==
          _)
        (:<
          _))
      (Variables|Default|SetOpened true)
      (Variables|/Game/Blueprints/GlobalInstance.GlobalInstance_C|SetPopupOpen _asglobal_instance true)
      (CallFunction|CheckSprite)
      (CallFunction|Popup)
      (CallFunction|Unlock)
      (bind _outactors (Actor|GetAllActorsOfClass "/Game/Blueprints/Calendar/SavingAndWidgets/BP_SaveDataActor.BP_SaveDataActor_C"))
      (Default|SaveGame _outactors))))

(event Custom|Set%20Status%20Closed
  ;[1 1 1] Closes the window
  (if (Variables|Default|GetOpened)
    (Variables|Default|SetOpened false)
    (bind _outactors (Actor|GetAllActorsOfClass "/Game/Blueprints/Calendar/SavingAndWidgets/BP_SaveDataActor.BP_SaveDataActor_C"))
    (Default|SaveGame _outactors)
    (CallFunction|CheckSprite)))

(event Custom|Load
  (bind _saveactor (Variables|Default|GetSaveActor))
  ;[1 1 1] Load
  (Utilities|Array|Clear (Variables|Default|GetSavedWindows))
  (Utilities|Array|Clear (Variables|Default|GetSaveStructure))
  (Utilities|Array|AppendArray (Variables|Default|GetSaveStructure) (Variables|/Game/Blueprints/Calendar/SavingAndWidgets/BP_SaveDataActor.BP_SaveDataActor_C|GetSAWindowStructure _saveactor))
  (Utilities|Array|AppendArray (Variables|Default|GetSavedWindows) (Variables|/Game/Blueprints/Calendar/SavingAndWidgets/BP_SaveDataActor.BP_SaveDataActor_C|GetSAWindows _saveactor))
  (Variables|Default|SetWindowStructure (Utilities|Struct|MakeWindowStructure (Utilities|Struct|BreakSaveWindowStructure (Utilities|Array|Get(acopy) (Variables|Default|GetSaveStructure) (Utilities|Array|FindItem (Variables|Default|GetSavedWindows) self)))))
  (Variables|Default|SetOpened (Utilities|Struct|BreakWindowStructure (Variables|Default|GetWindowStructure)))
  (Math|Integer|CompareInt (Class|KismetMathLibrary|GetMonth (Class|KismetMathLibrary|Today)) 11
    (:>
      _)
    (:==
      _)
    (:<
      _))
  (CallFunction|CheckSprite))

(event Custom|Check%20Sprite
  ;[1 1 1] Determines the correct sprite
  (if (Variables|Default|GetOpened)
    (Variables|Default|SetSpriteToUse (Variables|Default|GetOpenedSprite))
    (else
      (Variables|Default|SetSpriteToUse (Variables|Default|GetClosedSprite))))
  (Rendering|Components|Sprite|SetSprite (Variables|Default|Getkuva) (Variables|Default|GetSpriteToUse)))

(event Custom|Popup
  (bind _popupexplosion (Variables|Default|GetPopupExplosion))
  ;[1 1 1] Puff
  (Audio|PlaySound2D "/Game/Sounds/Effects/snd_crate_open.snd_crate_open" 1.0 1.0 0.0 0 0)
  (Rendering|SetVisibility _popupexplosion true false)
  (Components|Timeline|PlayfromStart _popupexplosion))

(event Custom|Save
  ;[1 1 1] Save
  (Variables|Default|SetWindowStructure (Utilities|Struct|MakeWindowStructure (Variables|Default|GetOpened))))

(event EventBeginPlay
  (bind _popupexplosion (Variables|Default|GetPopupExplosion))
  ;[1 1 1] Puff
  (Rendering|SetVisibility _popupexplosion false false)
  (Components|Timeline|SetLooping _popupexplosion false)
  (Rendering|Components|TextRender|SetText (Variables|Default|GetNumber) (Utilities|Text|ToText(Integer) (Variables|Default|GetOpeningDay)))
  (if (not (Variables|Default|GetShowNumber))
    (Rendering|SetVisibility (Variables|Default|GetNumber) false false)
    (Rendering|SetTranslucentSortPriority (Variables|Default|Getkuva) 100)))

(event EventActorOnInputTouchEnd
  (params (FingerIndex :type ETouchIndex%20Enum :default "Touch1"))
  (bind _returnvalue (Class|KismetMathLibrary|Today))
  ;[1 1 1] Opening
  (Math|Integer|CompareInt (Class|KismetMathLibrary|GetMonth _returnvalue) 11
    (:>
      _)
    (:==
      _)
    (:<
      _))
  (Math|Integer|CompareInt (Class|KismetMathLibrary|GetDay _returnvalue) (Variables|Default|GetOpeningDay)
    (:>
      _)
    (:==
      _))
  (CallFunction|SetStatusOpened))

(fn ConstructionScript)
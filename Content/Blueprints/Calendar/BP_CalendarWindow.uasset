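; Tappable advent calendar window actor that opens once the current day reaches its OpeningDay.
; A touch in November closes it; other months run the day check, with pre-November touches also printing an unlock notice.
; Opening or closing triggers a save through BP_SaveDataActor and a sprite check, which applies only the open sprite.
; Load restores Opened by the window's index in the saved arrays, then closes it through November.
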(event Custom|Save
  ;[1 1 1] Save
  (Variables|Default|SetWindowStructure (Utilities|Struct|MakeWindowStructure (Variables|Default|GetOpened))))

(event Custom|Set%20Status%20Opened
  ;[1 1 1] Opens the window
  (if (Variables|Default|GetOpened)
    (Development|PrintString "It's already open" true true "(R=1.000000,G=0.062022,B=0.000000,A=1.000000)")
    (else
      (Variables|Default|SetOpened true)
      (bind _outactors (Actor|GetAllActorsOfClass "/Game/Blueprints/Calendar/BP_SaveDataActor.BP_SaveDataActor_C"))
      (Default|SaveGame _outactors)
      (CallFunction|CheckSprite))))

(event Custom|Set%20Status%20Closed
  ;[1 1 1] Closes the window
  (if (Variables|Default|GetOpened)
    (Variables|Default|SetOpened false)
    (bind _outactors (Actor|GetAllActorsOfClass "/Game/Blueprints/Calendar/BP_SaveDataActor.BP_SaveDataActor_C"))
    (Default|SaveGame _outactors)
    (CallFunction|CheckSprite)
    (else
      (Development|PrintString "It's already closed" true true "(R=1.000000,G=0.038955,B=0.000000,A=1.000000)"))))

(event Custom|Load
  (bind _saveactor (Variables|Default|GetSaveActor))
  ;[1 1 1] Load
  (Utilities|Array|Clear (Variables|Default|GetSavedWindows))
  (Utilities|Array|Clear (Variables|Default|GetSaveStructure))
  (Utilities|Array|AppendArray (Variables|Default|GetSaveStructure) (Variables|/Game/Blueprints/Calendar/BP_SaveDataActor.BP_SaveDataActor_C|GetSAWindowStructure _saveactor))
  (Utilities|Array|AppendArray (Variables|Default|GetSavedWindows) (Variables|/Game/Blueprints/Calendar/BP_SaveDataActor.BP_SaveDataActor_C|GetSAWindows _saveactor))
  (Variables|Default|SetWindowStructure (Utilities|Struct|MakeWindowStructure (Utilities|Struct|BreakSaveWindowStructure (Utilities|Array|Get(acopy) (Variables|Default|GetSaveStructure) (Utilities|Array|FindItem (Variables|Default|GetSavedWindows) self)))))
  (Variables|Default|SetOpened (Utilities|Struct|BreakWindowStructure (Variables|Default|GetWindowStructure)))
  (Math|Integer|CompareInt (Class|KismetMathLibrary|GetMonth (Class|KismetMathLibrary|Today)) 11
    (:==
      _)
    (:<
      _))
  (CallFunction|SetStatusClosed)
  (CallFunction|CheckSprite))

(event Custom|Check%20Sprite
  ;[1 1 1] Determines the correct sprite
  (if (Variables|Default|GetOpened)
    (bind _output_get (Variables|Default|SetSpriteToUse "/Game/Sprites/xmaswindowopen_Sprite.xmaswindowopen_Sprite"))
    (Rendering|Components|Sprite|SetSprite (Variables|Default|Getkuva) _output_get)
    (else
      (Variables|Default|SetSpriteToUse "/Game/Sprites/xmas_window_Sprite.xmas_window_Sprite"))))

(event EventActorOnInputTouchBegin
  (params (FingerIndex :type ETouchIndex%20Enum :default "Touch1"))
  (bind _returnvalue (Class|KismetMathLibrary|Today))
  ;[1 1 1] Opening
  (Math|Integer|CompareInt (Class|KismetMathLibrary|GetMonth _returnvalue) 11
    (:>
      (Math|Integer|CompareInt (Class|KismetMathLibrary|GetDay _returnvalue) (Variables|Default|GetOpeningDay) :!label _label
        (:>
          (CallFunction|SetStatusOpened :!label _label_2))
        (:==
          (goto _label_2))
        (:<
          (Development|PrintString "Not today, mate"))))
    (:==
      (CallFunction|SetStatusClosed))
    (:<
      (Development|PrintString "unlocks comin in dec")
      (goto _label))))

(fn ConstructionScript)
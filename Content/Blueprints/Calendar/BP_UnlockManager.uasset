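; BP_UnlockManager tracks calendar unlock progress through the completed-day count held on the GlobalInstance game instance.
; On BeginPlay it caches the first GameManager in the level and reads CompletedDays into LastUnlockedDay.
; SetUnlockedDay adds the given day count to CompletedDays, rather than overwriting it, and prints the total for debugging.
; ScoreEtc copies the GameManager's current score into PresentScore.
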(event Custom|ScoreEtc
  (Variables|Default|SetpresentScore (Variables|/Game/Blueprints/Main/GameManager.GameManager_C|GetScore (stale EventBeginPlay _output_get))))

(event EventBeginPlay
  (bind _asglobal_instance (Utilities|Casting|CastToGlobalInstance (Game|GetGameInstance)))
  (bind _outactors (Actor|GetAllActorsOfClass "/Game/Blueprints/Main/GameManager.GameManager_C"))
  (bind _output_get (Variables|Default|SetGameManager (Utilities|Array|Get(acopy) _outactors)))
  (Variables|Default|SetlastUnlockedDay (Variables|/Game/Blueprints/GlobalInstance.GlobalInstance_C|GetCompletedDays _asglobal_instance)))

(event EventSetUnlockedDay
  (params (dayCount :type Integer%20%28by%20ref%29))
  (bind _asglobal_instance (Utilities|Casting|CastToGlobalInstance (Game|GetGameInstance)))
  (bind _output_get (Variables|/Game/Blueprints/GlobalInstance.GlobalInstance_C|SetCompletedDays _asglobal_instance (+ (Variables|/Game/Blueprints/GlobalInstance.GlobalInstance_C|GetCompletedDays _asglobal_instance) dayCount)))
  (Development|PrintString (Utilities|String|ToString(Integer) _output_get) true false "(R=0.000000,G=0.660000,B=1.000000,A=1.000000)" 3.0)
  (Development|PrintString "Completed days"))

(fn ConstructionScript)
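; Actor that saves and loads the calendar's progress through a BP_SaveData object in the "Calendar" slot.
; Saving recreates the slot from GlobalInstance unlocks and progress, the highscore, today's day and each calendar window's state, writing to disk once per window.
; Loading restores GlobalInstance stats, caches the remaining data on itself, then hands each window a self-reference and calls its Load.
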(event Custom|SaveGame
  ;[1 1 1] Save
  (bind _returnvalue (SaveGame|DoesSaveGameExist "Calendar"))
  (if _returnvalue
    (SaveGame|DeleteGameinSlot "Calendar"))
  (bind _returnvalue_2 (SaveGame|CreateSaveGameObject "/Game/Blueprints/Calendar/SavingAndWidgets/BP_SaveData.BP_SaveData_C"))
  (Variables|Default|SetSaveReference _returnvalue_2)
  (bind _asbp_save_data (Utilities|Casting|CastToBP_SaveData (Variables|Default|GetSaveReference)))
  (CallFunction|SaveGlobalVariables _asbp_save_data)
  (bind _outactors (Actor|GetAllActorsOfClass "/Game/Blueprints/Calendar/BP_CalenderWindow.BP_CalenderWindow_C"))
  (for _array_element _outactors
    (Default|Save _array_element)
    (Utilities|Array|Add (Variables|/Game/Blueprints/Calendar/SavingAndWidgets/BP_SaveData.BP_SaveData_C|GetWindowsStructure _asbp_save_data) (Utilities|Struct|MakeSaveWindowStructure (Utilities|Struct|BreakWindowStructure (Variables|/Game/Blueprints/Calendar/BP_CalenderWindow.BP_CalenderWindow_C|GetWindowStructure _array_element))))
    (Utilities|Array|Add (Variables|/Game/Blueprints/Calendar/SavingAndWidgets/BP_SaveData.BP_SaveData_C|GetWindows _asbp_save_data) _array_element)
    (SaveGame|SaveGametoSlot (Variables|Default|GetSaveReference) "Calendar")))

(event Custom|LoadGame
  ;[1 1 1] Load
  (bind _returnvalue (SaveGame|DoesSaveGameExist "Calendar"))
  (if _returnvalue
    (bind _returnvalue_2 (SaveGame|LoadGamefromSlot "Calendar"))
    (bind _asbp_save_data (Utilities|Casting|CastToBP_SaveData _returnvalue_2))
    (bind _asglobal_instance (Utilities|Casting|CastToGlobalInstance (Game|GetGameInstance)))
    (Default|LoadStats _asglobal_instance (Variables|/Game/Blueprints/Calendar/SavingAndWidgets/BP_SaveData.BP_SaveData_C|GetChimneys _asbp_save_data) (Variables|/Game/Blueprints/Calendar/SavingAndWidgets/BP_SaveData.BP_SaveData_C|GetVisuals _asbp_save_data) (Variables|/Game/Blueprints/Calendar/SavingAndWidgets/BP_SaveData.BP_SaveData_C|GetSavedScore _asbp_save_data) (Variables|/Game/Blueprints/Calendar/SavingAndWidgets/BP_SaveData.BP_SaveData_C|GetMaps _asbp_save_data) (Variables|/Game/Blueprints/Calendar/SavingAndWidgets/BP_SaveData.BP_SaveData_C|GetCompletedDays _asbp_save_data) (Variables|/Game/Blueprints/Calendar/SavingAndWidgets/BP_SaveData.BP_SaveData_C|GetPresentUnlocks _asbp_save_data))
    (Variables|Default|SetSAHighscore (Variables|/Game/Blueprints/Calendar/SavingAndWidgets/BP_SaveData.BP_SaveData_C|GetHighscore _asbp_save_data))
    (Variables|Default|SetSALastVisit (Variables|/Game/Blueprints/Calendar/SavingAndWidgets/BP_SaveData.BP_SaveData_C|GetLastSavedVisit _asbp_save_data))
    (Utilities|Array|AppendArray (Variables|Default|GetSAWindows) (Variables|/Game/Blueprints/Calendar/SavingAndWidgets/BP_SaveData.BP_SaveData_C|GetWindows _asbp_save_data))
    (Utilities|Array|AppendArray (Variables|Default|GetSAWindowStructure) (Variables|/Game/Blueprints/Calendar/SavingAndWidgets/BP_SaveData.BP_SaveData_C|GetWindowsStructure _asbp_save_data))
    (bind _outactors (Actor|GetAllActorsOfClass "/Game/Blueprints/Calendar/BP_CalenderWindow.BP_CalenderWindow_C"))
    (for _array_element _outactors
      (Variables|/Game/Blueprints/Calendar/BP_CalenderWindow.BP_CalenderWindow_C|SetSaveActor _array_element self)
      (Default|Load _array_element))
    (else
      (Development|PrintString "Save Missing!"))))

(event Custom|Save%20Global%20Variables
  (params (SaveData :type BP%20Save%20Data%20Object%20Reference))
  ;[1 1 1] Save From GlobalInstance
  (bind _asglobal_instance (Utilities|Casting|CastToGlobalInstance (Game|GetGameInstance)))
  (Variables|/Game/Blueprints/Calendar/SavingAndWidgets/BP_SaveData.BP_SaveData_C|SetChimneys SaveData (Variables|/Game/Blueprints/GlobalInstance.GlobalInstance_C|GetChimneyUnlocks _asglobal_instance))
  (Variables|/Game/Blueprints/Calendar/SavingAndWidgets/BP_SaveData.BP_SaveData_C|SetVisuals SaveData (Variables|/Game/Blueprints/GlobalInstance.GlobalInstance_C|GetVisualUpgrades _asglobal_instance))
  (Variables|/Game/Blueprints/Calendar/SavingAndWidgets/BP_SaveData.BP_SaveData_C|SetSavedScore SaveData (Variables|/Game/Blueprints/GlobalInstance.GlobalInstance_C|GetSavedScore _asglobal_instance))
  (Variables|/Game/Blueprints/Calendar/SavingAndWidgets/BP_SaveData.BP_SaveData_C|SetMaps SaveData (Variables|/Game/Blueprints/GlobalInstance.GlobalInstance_C|GetMapsUnlocked _asglobal_instance))
  (Variables|/Game/Blueprints/Calendar/SavingAndWidgets/BP_SaveData.BP_SaveData_C|SetCompletedDays SaveData (Variables|/Game/Blueprints/GlobalInstance.GlobalInstance_C|GetCompletedDays _asglobal_instance))
  (Variables|/Game/Blueprints/Calendar/SavingAndWidgets/BP_SaveData.BP_SaveData_C|SetLastSavedVisit SaveData (Class|KismetMathLibrary|GetDay (Class|KismetMathLibrary|Today)))
  (Variables|/Game/Blueprints/Calendar/SavingAndWidgets/BP_SaveData.BP_SaveData_C|SetHighscore SaveData (Variables|Default|GetSAHighscore))
  (Variables|/Game/Blueprints/Calendar/SavingAndWidgets/BP_SaveData.BP_SaveData_C|SetPresentUnlocks SaveData (Variables|/Game/Blueprints/GlobalInstance.GlobalInstance_C|GetPresentUnlocks _asglobal_instance)))

(fn ConstructionScript)
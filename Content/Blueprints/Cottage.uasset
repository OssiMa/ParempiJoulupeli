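; Cottage is a moving house actor that serves as a chimney delivery target for gifts.
; Each tick it slides along world X at MoveSpeed, scaled by delta time, without sweeping.
; When an actor tagged Gift overlaps it, it destroys the gift and its own BoxTrigger component, then increments PresentsDelivered on the first GameDataStorage actor found in the level.
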(event EventTick
  (params (DeltaSeconds :type Float%20%28single-precision%29))
  (bind _returnvalue (Transformation|GetActorTransform))
  (bind _returnvalue_2 (Math|Transform|TransformLocation _returnvalue "0, 0, 0"))
  (bind (_x _y _z) (Math|Vector|BreakVector _returnvalue_2))
  ;[1 1 1] House movement
  (Transformation|SetActorLocation (Math|Vector|MakeVector (+ (* DeltaSeconds (Variables|Default|GetMoveSpeed)) _x) _y _z) false false))

(event Collision|EventActorBeginOverlap
  (params (OtherActor :type Actor%20Object%20Reference))
  ;[1 1 1] Chimney
  (if (Actor|ActorHasTag OtherActor "Gift")
    (Actor|DestroyActor OtherActor)
    (Components|DestroyComponent (Variables|Default|GetBoxTrigger))
    (bind _outactors (Actor|GetAllActorsOfClass "/Game/Blueprints/GameDataStorage.GameDataStorage_C"))
    (Variables|/Game/Blueprints/GameDataStorage.GameDataStorage_C|SetPresentsDelivered (Utilities|Array|Get(acopy) _outactors) (+ (Variables|/Game/Blueprints/GameDataStorage.GameDataStorage_C|GetPresentsDelivered (Utilities|Array|Get(acopy) _outactors)) 1))))

(fn ConstructionScript)
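; BP_HouseSpawner is a house spawner actor that holds spawn permission and hooks into shared difficulty settings on the GlobalInstance game instance.
; On BeginPlay it caches the GlobalInstance and calls UnlockHarderDifficulty if increased house spawns are flagged there.
; Events toggle the CanSpawn flag and add to the global SpeedModifier.
; The spawn logic itself is not in these graphs.
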(event Custom|Don'tAllowSpawning
  (Variables|Default|SetcanSpawn false))

(event Custom|AllowSpawning
  (Variables|Default|SetcanSpawn true))

(event EventApplySpeedModifier
  (params (speed :type Float%20%28single-precision%29%20%28by%20ref%29))
  (Variables|/Game/Blueprints/GlobalInstance.GlobalInstance_C|SetSpeedModifier (stale EventBeginPlay _asglobal_instance) (+ (Variables|/Game/Blueprints/GlobalInstance.GlobalInstance_C|GetSpeedModifier (stale EventBeginPlay _asglobal_instance)) speed)))

(event Collision|EventActorBeginOverlap
  (params (OtherActor :type Actor%20Object%20Reference)))

(event EventTick
  (params (DeltaSeconds :type Float%20%28single-precision%29)))

(event EventBeginPlay
  (bind _asglobal_instance (Utilities|Casting|CastToGlobalInstance (Game|GetGameInstance)))
  (if (Variables|/Game/Blueprints/GlobalInstance.GlobalInstance_C|GetIncreaseHouseSpawns _asglobal_instance)
    (Class|HouseSpawner|UnlockHarderDifficulty 1.0)))

(fn ConstructionScript)
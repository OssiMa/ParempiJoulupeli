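; CameraTest is a touch-swipe camera test that slides its actor along world X as a finger drags horizontally.
; The touch-move event records the active finger, and Tick polls its state, storing the screen X when a press begins.
; While held, the inverted, scaled delta offsets the actor's X, applying the move and updating the stored X only when the result lies strictly between MaxLeft and MaxRight.
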(event EventTick
  (params (DeltaSeconds :type Float%20%28single-precision%29))
  (bind _returnvalue (Game|GetPlayerController 0))
  (bind _returnvalue_2 (Transformation|GetActorTransform))
  (bind _touchinput (Variables|Default|GettouchInput))
  (bind (_locationx _locationy _biscurrentlypressed) (Class|PlayerController|GetInputTouchState _returnvalue _touchinput))
  (bind _returnvalue_3 (Math|Transform|TransformLocation _returnvalue_2 "0, 0, 0"))
  (bind (_x _y _z) (Math|Vector|BreakVector _returnvalue_3))
  ;[1 1 1] Camera swipe
  (if _biscurrentlypressed
    (if (Variables|Default|Gettouched)
      (Math|Float|CompareFloat (Variables|Default|GetMaxLeft) (+ (* (- _locationx (Variables|Default|GetX)) -2.0) _x)
        (:<
          (Math|Float|CompareFloat (Variables|Default|GetMaxRight) (+ (* (- _locationx (Variables|Default|GetX)) -2.0) _x)
            (:>
              (Transformation|SetActorLocation (Math|Vector|MakeVector (+ (* (- _locationx (Variables|Default|GetX)) -2.0) _x) _y _z) false false)
              (Variables|Default|SetX _locationx)))))
      (else
        (Variables|Default|Settouched true)
        (Variables|Default|SetX _locationx)))
    (else
      (Variables|Default|Settouched false))))

(event Input|TouchEvents|InputTouch
  (params (Location :type Vector) (FingerIndex :type ETouchIndex%20Enum))
  ;[1 1 1] Camera swipe
  (:Moved
    (Variables|Default|SettouchInput FingerIndex)))

(fn ConstructionScript)